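; Player controller that manages the player character's HUD, automatic respawn and pause menu input.
; On possessing a BP_PlayerCharacter, it saves the pawn's transform, binds its destroyed event, creates the W_HUD widget and routes health component changes to it.
; When the pawn is destroyed, it waits briefly, spawns and possesses a new character at the saved transform, then resets and rebinds the health display.
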(event Custom|OnPawnDestroyer
  (params (DestroyedActor :type Actor%20Object%20Reference))
  ;[1 1 1] Player Exist?
  (Utilities|FlowControl|Delay 2.0)
  (CallFunction|Respawn))

(event Custom|Respawn
  ;[1 1 1] Respawn
  (bind _returnvalue (Game|SpawnActorfromClass "/Game/PlayerCharacter/BP_PlayerCharacter.BP_PlayerCharacter_C" (Variables|Default|GetInicjalTransform) "Undefined" "MultiplyWithRoot" 0 0))
  (Pawn|Possess _returnvalue)
  (Utilities|IsValid _returnvalue
    (:Is%20Valid
      (Game|BindEventtoOnDestroyed (delegate Custom|OnPawnDestroyer))
      (Default|SetHealth (Variables|Default|GetHUD) 1.0 1.0)
      (CallFunction|BindtoHealthChanges))))

(event Custom|Setup%20HUD
  ;[1 1 1] Set up HUD
  (bind _returnvalue (UserInterface|CreateWidget "/Game/Blueprint/Widgets/W_HUD.W_HUD_C"))
  (Variables|Default|SetHUD _returnvalue)
  (UserInterface|Viewport|AddtoViewport _returnvalue 0)
  (CallFunction|BindtoHealthChanges))

(event Custom|Set%20Health
  (params (CurrentHealth :type Float%20%28double-precision%29) (MaxHealth :type Float%20%28double-precision%29))
  ;[1 1 1] Set up HUD
  (Default|SetHealth (Variables|Default|GetHUD) CurrentHealth MaxHealth))

(event Custom|Bind%20to%20Health%20changes
  ;[1 1 1] Set up HUD
  (bind _asbp_player_character (Utilities|Casting|CastToBP_PlayerCharacter (Pawn|GetControlledPawn)))
  (EventDispatchers|BindEventtoOnHealthChanged (Variables|/Game/PlayerCharacter/BP_PlayerCharacter.BP_PlayerCharacter_C|GetBP_HealthComponent _asbp_player_character) (delegate Custom|Set%20Health)))

(event EventPossess
  (params (PossessedPawn :type Pawn%20Object%20Reference))
  ;[1 1 1] Player Exist?
  (bind _asbp_player_character (Utilities|Casting|CastToBP_PlayerCharacter PossessedPawn))
  (bind _output_get (Variables|Default|SetAs%20BP%20Player%20Character _asbp_player_character))
  (Utilities|IsValid _output_get
    (:Is%20Valid
      (Variables|Default|SetInicjalTransform (Transformation|GetActorTransform _output_get))
      (Game|BindEventtoOnDestroyed _output_get (delegate Custom|OnPawnDestroyer))
      (CallFunction|SetupHUD))))

(event Input|ActionEvents|InputActionPauseMenu
  (params (Key :type Key%20Structure :default "None"))
  ;[1 1 1] Pause Menu
  (:Pressed
    (bind _hud (Variables|Default|GetHUD)
      (:then
        (Default|TooglePauseMenu _hud))
      (:else))))

(fn ConstructionScript)