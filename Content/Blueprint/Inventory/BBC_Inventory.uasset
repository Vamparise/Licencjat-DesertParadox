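; BBC_Inventory is an inventory component for the player that records collected items and shows them in the UI.
; AddItemsToInventory adds the item's enum value to an inventory collection.
; It then casts the owner to BP_PlayerCharacter and passes the item name and enum to that character's InventoryWidget list.
; An older branch storing items in a separate Inventory variable is left unconnected.
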(fn AddItemstoInventory
  (params (NewItem :type String%20%28by%20ref%29) (NewItem1 :type E_Notes%20Enum%20%28by%20ref%29 :default "NewEnumerator0"))
  (Utilities|Array|Add (Variables|Default|GetInventory_0) NewItem1)
  (bind _asbp_player_character (Utilities|Casting|CastToBP_PlayerCharacter (Components|GetOwner)))
  (Default|AddItemtoList (Variables|/Game/PlayerCharacter/BP_PlayerCharacter.BP_PlayerCharacter_C|GetInventoryWidget _asbp_player_character) NewItem NewItem1))