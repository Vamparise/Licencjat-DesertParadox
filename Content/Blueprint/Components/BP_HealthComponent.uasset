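; Health component that tracks its owner's hit points, starting at max on BeginPlay and reduced through the owner's any-damage event.
; Damage is clamped and broadcast through OnHealthChanged; at zero it fires OnHealthDepleted and destroys the owner.
; Otherwise a retriggerable delay starts a timed regeneration loop that adds health in steps until reaching max, without clamping overshoot.
; Debug print handlers exist, but their bindings never run.
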(event Custom|RegenerationHealth
  ;[1 1 1] RegenerationHealth
  (Utilities|FlowControl|RetriggerableDelay 2.0)
  (Variables|Default|SetCanRegenerateHealth true)
  (if (not (== (Variables|Health|GetCurrentHitPoints) (Variables|Health|GetMaxHealth))) :!label _label
    (Utilities|FlowControl|Delay 0.2)
    (Variables|Health|SetCurrentHitPoints (+ (Variables|Health|GetCurrentHitPoints) 1e+01))
    (Default|CallOnHealthChanged (Variables|Health|GetCurrentHitPoints) (Variables|Health|GetMaxHealth))
    (if (Variables|Default|GetCanRegenerateHealth)
      (if (>= (Variables|Health|GetCurrentHitPoints) (Variables|Health|GetMaxHealth))
        (if (not (== (Variables|Health|GetCurrentHitPoints) (Variables|Health|GetMaxHealth)))
          (Variables|Default|SetMax%20Health (Variables|Health|GetMaxHealth)))
        (else
          (goto _label))))
    (else
      (Variables|Default|SetCanRegenerateHealth false))))

(event Custom|Test
  ;[1 1 1] Test
)

(event Custom|OnDeath
  ;[1 1 1] Test
  (Development|PrintString "Character is Death" true true "(R=0.338856,G=1.000000,B=0.000000,A=1.000000)" 5.0))

(event Custom|OnDamageTest
  (params (CurrentHealth :type Float%20%28double-precision%29) (MaxHealth :type Float%20%28double-precision%29))
  ;[1 1 1] Test
  (Development|PrintString (Utilities|String|Append "Health: " (Utilities|String|ToString(Float) (Variables|Health|GetCurrentHitPoints))) true true "(R=0.000000,G=0.660000,B=1.000000,A=1.000000)" 3.0))

(event Custom|OnDamageTaken
  (params (DamagedActor :type Actor%20Object%20Reference) (Damage :type Float%20%28single-precision%29) (DamageType :type Damage%20Type%20Object%20Reference) (InstigatedBy :type Controller%20Object%20Reference) (DamageCauser :type Actor%20Object%20Reference))
  (bind _returnvalue (Components|GetOwner))
  ;[1 1 1] Handle Damage
  (Variables|Health|SetCurrentHitPoints (Math|Float|Clamp(Float) (- (Variables|Health|GetCurrentHitPoints) Damage) 0.0 (Variables|Health|GetMaxHealth)))
  (Default|CallOnHealthChanged (Variables|Health|GetCurrentHitPoints) (Variables|Health|GetMaxHealth))
  (if (<= (Variables|Health|GetCurrentHitPoints) 0.0)
    (Default|CallOnHealthDepleted)
    (Utilities|IsValid _returnvalue
      (:Is%20Valid
        (Actor|DestroyActor _returnvalue)))
    (else
      (CallFunction|RegenerationHealth))))

(event EventBeginPlay
  (bind _returnvalue (Components|GetOwner))
  ;[1 1 1] TestDamage
  (Variables|Health|SetCurrentHitPoints (Variables|Health|GetMaxHealth))
  (Utilities|IsValid _returnvalue
    (:Is%20Valid
      (EventDispatchers|BindEventtoOnTakeAnyDamage _returnvalue (delegate Custom|OnDamageTaken))
      (CallFunction|Test))))