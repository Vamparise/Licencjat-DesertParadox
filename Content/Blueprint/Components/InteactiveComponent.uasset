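; Interaction logic, named as a component, that lets the player use the actor under the camera's view with the E key.
; Each tick, a debug-drawn line trace runs forward from the camera and stores any hit actor without filtering.
; Pressing E sends that actor an InteractWith message with the player character.
; A hit shows a prompt widget through a never-reset DoOnce, and a miss removes it.
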(event EventBeginPlay)

(event EventTick
  (params (DeltaSeconds :type Float%20%28single-precision%29))
  (CallFunction|Interactive))

(event Input|KeyboardEvents|E
  (params (Key :type Key%20Structure :default "None"))
  (:Pressed
    (bind _hit_actor (Variables|Default|GetHit%20Actor)
      (:then
        (Class|ObjectInteactive|Interactwith(Message) _hit_actor (.AsBP%20Player%20Character (Utilities|Casting|CastToBP_PlayerCharacter (Game|GetPlayerCharacter 0)))))
      (:else))))

(fn Interactive
  (bind _returnvalue (Game|GetPlayerCameraManager 0))
  (bind _returnvalue_2 (Transformation|GetActorLocation _returnvalue))
  (bind (_outhit _returnvalue_3) (Collision|LineTraceByChannel _returnvalue_2 (+ _returnvalue_2 (* (Math|Vector|GetForwardVector (Camera|GetCameraRotation _returnvalue)) "500.000000,500.000000,500.000000")) "TraceTypeQuery3" false 0 "ForOneFrame"))
  (Variables|Default|SetOut%20Hit _outhit)
  (if _returnvalue_3
    (Variables|Default|SetHit%20Actor (.HitActor (Collision|BreakHitResult _outhit)))
    (CallFunction|WidgetInteracive)
    (else
      (Variables|Default|SetHit%20Actor 0)
      (bind _widget (Variables|Default|GetWidget)
        (:then
          (Widget|RemovefromParent _widget)
          (Development|PrintString "Remove E"))
        (:else)))))

(fn WidgetInteracive
  (Utilities|FlowControl|DoOnce false
    (:Completed
      (bind _returnvalue (UserInterface|CreateWidget "/Game/Blueprint/Widgets/W_Interactive.W_Interactive_C"))
      (bind _output_get (Variables|Default|SetWidget _returnvalue))
      (UserInterface|Viewport|AddtoViewport _output_get 0)
      (Development|PrintString "eqweqwe"))))