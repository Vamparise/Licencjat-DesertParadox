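; BP_BasicColider is a level gameplay trigger that reports when something enters or leaves its Box component.
; BeginPlay binds the box's begin and end overlap events to handlers that print the overlapping actor's name.
; The handlers then call OnPawnEnter and OnPawnLeave so other logic can react.
; Despite those names, neither handler checks that the overlapping actor is a Pawn.
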(event Custom|On%20Begin%20Box%20Overlap
  (params (OverlappedComponent :type Primitive%20Component%20Object%20Reference) (OtherActor :type Actor%20Object%20Reference) (OtherComp :type Primitive%20Component%20Object%20Reference) (OtherBodyIndex :type Integer) (bFromSweep :type Boolean) (SweepResult :type Hit%20Result%20Structure%20%28by%20ref%29))
  ;[1 1 1] Box Begin overlap
  (Development|PrintString (Utilities|String|Append "Box Begin Overlap" (Utilities|GetDisplayName OtherActor)))
  (Default|CallOnPawnEnter))

(event Custom|Box%20End%20Overlap
  (params (OverlappedComponent :type Primitive%20Component%20Object%20Reference) (OtherActor :type Actor%20Object%20Reference) (OtherComp :type Primitive%20Component%20Object%20Reference) (OtherBodyIndex :type Integer))
  ;[1 1 1] Box End Overlap
  (Development|PrintString (Utilities|String|Append "Box End Overlap" (Utilities|GetDisplayName OtherActor)))
  (Default|CallOnPawnLeave))

(event EventBeginPlay
  ;[1 1 1] Box Begin overlap
  (Collision|BindEventtoOnComponentBeginOverlap (Variables|Default|GetBox) (delegate Custom|On%20Begin%20Box%20Overlap))
  ;[1 1 1] Box End Overlap
  (Collision|BindEventtoOnComponentEndOverlap (Variables|Default|GetBox) (delegate Custom|Box%20End%20Overlap)))

(event Collision|EventActorBeginOverlap
  (params (OtherActor :type Actor%20Object%20Reference)))

(event EventTick
  (params (DeltaSeconds :type Float%20%28single-precision%29)))

(fn ConstructionScript)