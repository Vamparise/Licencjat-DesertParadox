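; Door Blueprint that shows or hides a flat cube panel in response to an optional linked sensor and switch (Interuptor).
; It appears on BeginPlay and binds to both devices' events.
; Pawn entry or switch deactivation shows it, while pawn exit or switch activation hides it.
; One timeline, played forward or reversed, animates the cube's width and height, with its Y scale held at zero.
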(event Custom|Appear
  (bind _scaletrack (Timeline|Timeline_AppearDissapear Play)
    (:Update
      (Transformation|SetWorldScale3D (Variables|Default|GetCube) (Math|Vector|MakeVector (* _scaletrack 2.0) 0.0 (* _scaletrack 3.0))))))

(event Custom|Dissappear
  (bind _scaletrack (Timeline|Timeline_AppearDissapear Reverse)
    (:Update
      (Transformation|SetWorldScale3D (Variables|Default|GetCube) (Math|Vector|MakeVector (* _scaletrack 2.0) 0.0 (* _scaletrack 3.0))))))

(event Custom|Pawn%20Enter
  ;[1 1 1] Sensor Activate
  (CallFunction|Appear))

(event Custom|Pawn%20Leave
  ;[1 1 1] Sensor Activate
  (CallFunction|Dissappear))

(event Custom|OnInterruptorActivated
  ;[1 1 1] Interruptor Activation
  (CallFunction|Dissappear))

(event Custom|OnInterruptorDeactivated
  ;[1 1 1] Interruptor Activation
  (CallFunction|Appear))

(event EventBeginPlay
  (CallFunction|Appear)
  (Utilities|FlowControl|Sequence
    (:then_0
      ;[1 1 1] Sensor Activate
      (bind _sensor (Variables|Default|GetSensor)
        (:then
          (EventDispatchers|BindEventtoOnPawnEnter _sensor (delegate Custom|Pawn%20Enter))
          (EventDispatchers|BindEventtoOnPawnLeave _sensor (delegate Custom|Pawn%20Leave)))
        (:else)))
    (:then_1
      ;[1 1 1] Interruptor Activation
      (bind _interuptor (Variables|Activation|GetInteruptor)
        (:then
          (EventDispatchers|BindEventtoOnInterruptorActivated _interuptor (delegate Custom|OnInterruptorActivated))
          (EventDispatchers|BindEventtoOnInterruptorDeactivated _interuptor (delegate Custom|OnInterruptorDeactivated)))
        (:else)))))

(fn ConstructionScript)