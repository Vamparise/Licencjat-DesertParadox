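; BP_SlowTrap is a level trap that slows the affected character by halving its max walk speed.
; ApplyEffect caches the CharacterMovement MaxWalkSpeed before reducing it, and RemoveEffect restores the cached value, both guarded by a validity check on AffectedCharacter.
; The file holds only this effect logic, with no triggering or timing, and its construction script just calls the parent.
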(event EventApplyEffect
  ;[1 1 1] VelocityTrapLogic
  (bind _affectedcharacter (Variables|Default|GetAffectedCharacter)
    (:then
      (bind _output_get (Variables|Default|SetOriginalWalkSpeed (Variables|/Script/Engine.CharacterMovementComponent|GetMaxWalkSpeed (Variables|/Script/Engine.Character|GetCharacterMovement _affectedcharacter))))
      (Variables|/Script/Engine.CharacterMovementComponent|SetMaxWalkSpeed (Variables|/Script/Engine.Character|GetCharacterMovement _affectedcharacter) (/ _output_get 2.0)))
    (:else)))

(event EventRemoveEffect
  ;[1 1 1] VelocityTrapLogic
  (bind _affectedcharacter (Variables|Default|GetAffectedCharacter)
    (:then
      (Variables|/Script/Engine.CharacterMovementComponent|SetMaxWalkSpeed (Variables|/Script/Engine.Character|GetCharacterMovement _affectedcharacter) (Variables|Default|GetOriginalWalkSpeed)))
    (:else)))

(fn ConstructionScript
  (|CallParentFunction))