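; Spike trap actor that applies damage to actors that begin overlapping its box and periodically toggles between shown and hidden.
; After an initial delay on BeginPlay, a looping timer flips BSpikesVisible and passes it to HideSpikes, so true actually means hidden.
; HideSpikes switches spike visibility and box collision together, using query-only collision when shown and none when hidden.
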(event OnComponentBeginOverlap(Box)
  (params (OverlappedComponent :type Primitive%20Component%20Object%20Reference) (OtherActor :type Actor%20Object%20Reference) (OtherComp :type Primitive%20Component%20Object%20Reference) (OtherBodyIndex :type Integer) (bFromSweep :type Boolean) (SweepResult :type Hit%20Result%20Structure%20%28by%20ref%29))
  ;[1 1 1] Do Damage
  (Game|Damage|ApplyDamage OtherActor (Variables|Damage|GetDamage) 0 0))

(event Custom|Hide%20Spikes
  (params (B_ShouldHide :type Boolean))
  (bind _spikes (Variables|Default|GetSpikes))
  (bind _box (Variables|Default|GetBox))
  ;[1 1 1] Show/Hide SPikes
  (if B_ShouldHide
    (Rendering|SetVisibility _spikes false true)
    (Collision|SetCollisionEnabled _box "NoCollision")
    (else
      (Rendering|SetVisibility _spikes true true)
      (Collision|SetCollisionEnabled _box "QueryOnly"))))

(event Custom|ToggleSpikes
  (Variables|Spikes|SetB_SpikesVisible (not (Variables|Spikes|GetB_SpikesVisible)))
  (CallFunction|HideSpikes (Variables|Spikes|GetB_SpikesVisible)))

(event EventBeginPlay
  (Utilities|FlowControl|Delay (Variables|Spikes|GetInititalDelay))
  (Utilities|Time|SetTimerbyEvent (delegate Custom|ToggleSpikes) (Variables|Spikes|GetSpikesTime) true))

(fn ConstructionScript)