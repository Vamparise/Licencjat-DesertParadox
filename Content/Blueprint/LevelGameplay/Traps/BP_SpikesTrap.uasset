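; Spike trap that pops up when the player stands in its trigger and damages actors that touch it.
; An actor overlap starts a delayed show-then-hide cycle that repeats while the player character stays inside TriggerBox.
; Spike visibility and damage Box collision switch together, and Box overlaps apply damage to any actor.
; HideSpikes always hides regardless of its argument, and the looping timer setup is disconnected.
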(event OnComponentBeginOverlap(Box)
  (params (OverlappedComponent :type Primitive%20Component%20Object%20Reference) (OtherActor :type Actor%20Object%20Reference) (OtherComp :type Primitive%20Component%20Object%20Reference) (OtherBodyIndex :type Integer) (bFromSweep :type Boolean) (SweepResult :type Hit%20Result%20Structure%20%28by%20ref%29))
  ;[1 1 1] Do Damage
  (Game|Damage|ApplyDamage OtherActor (Variables|Damage|GetDamage) 0 0))

(event Custom|Hide%20Spikes
  (params (B_ShouldHide :type Boolean))
  ;[1 1 1] Show/Hide SPikes
  (Rendering|SetVisibility (Variables|Default|GetSpikes) false true)
  (Collision|SetCollisionEnabled (Variables|Default|GetBox) "NoCollision"))

(event Custom|ToggleSpikes
  (Variables|Spikes|SetB_SpikesVisible (not (Variables|Spikes|GetB_SpikesVisible)))
  (CallFunction|HideSpikes (Variables|Spikes|GetB_SpikesVisible)))

(event EventBeginPlay
  (CallFunction|HideSpikes false))

(event Collision|EventActorBeginOverlap
  (params (OtherActor :type Actor%20Object%20Reference))
  (bind _spikes (Variables|Default|GetSpikes))
  (bind _box (Variables|Default|GetBox))
  ;[1 1 1] Show/Hide SPikes
  (if (Collision|IsOverlappingActor (Variables|Default|GetTriggerBox) (Game|GetPlayerCharacter 0) :!class /Script/Engine.PrimitiveComponent) :!label _label
    (Utilities|FlowControl|Delay (Variables|Default|GetDelaySpikes))
    (Rendering|SetVisibility _spikes true true)
    (Collision|SetCollisionEnabled _box "QueryOnly")
    (Utilities|FlowControl|Delay (Variables|Default|GetDurationVisible))
    (CallFunction|HideSpikes false)
    (goto _label)
    (else
      (Rendering|SetVisibility _spikes false true)
      (Collision|SetCollisionEnabled _box "NoCollision"))))

(fn ConstructionScript)