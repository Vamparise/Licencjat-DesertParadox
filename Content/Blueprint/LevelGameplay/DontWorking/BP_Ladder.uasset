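; BP_Ladder is a procedurally built ladder actor with a climb-check box, intended for player climbing.
; Its construction script stacks section meshes by rung count at a hardcoded 56-unit spacing, leaving the computed mesh height unused.
; It then sizes and positions the PlayerClimbCheck box to span the stack.
; Both overlap events are empty, so the ToggleClimbing calls on BP_PlayerCharacter are disconnected and never run.
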(event OnComponentBeginOverlap(PlayerClimbCheck)
  (params (OverlappedComponent :type Primitive%20Component%20Object%20Reference) (OtherActor :type Actor%20Object%20Reference) (OtherComp :type Primitive%20Component%20Object%20Reference) (OtherBodyIndex :type Integer) (bFromSweep :type Boolean) (SweepResult :type Hit%20Result%20Structure%20%28by%20ref%29)))

(event OnComponentEndOverlap(PlayerClimbCheck)
  (params (OverlappedComponent :type Primitive%20Component%20Object%20Reference) (OtherActor :type Actor%20Object%20Reference) (OtherComp :type Primitive%20Component%20Object%20Reference) (OtherBodyIndex :type Integer)))

(event EventBeginPlay)

(event Collision|EventActorBeginOverlap
  (params (OtherActor :type Actor%20Object%20Reference)))

(event EventTick
  (params (DeltaSeconds :type Float%20%28single-precision%29)))

(fn ConstructionScript
  (bind _playerclimbcheckboxsizexy (Variables|LaddetStepUp|GetPlayerClimbCheckBoxSizeXY))
  (bind _returnvalue (/ _playerclimbcheckboxsizexy 2.0))
  (Utilities|FlowControl|Sequence
    (:then_0
      (Variables|LaddetStepUp|SetLadderSectionMeshHeight (* (.z (.boxextent (StaticMesh|GetBounds (Variables|LaddetStepUp|GetLaddeSectionMesh)))) 2.0)))
    (:then_1
      (for _index (range 0 (- (Variables|LaddetStepUp|GetNumberOfRungs) 1))
        (bind _returnvalue_2 (AddComponent|AddStaticMeshComponent false (Math|Transform|MakeTransform (Math|Vector|MakeVector 0.0 0.0 (Math|Conversions|ToFloat(Integer) (* _index 56))) "0, 0, 0" "1.000000,1.000000,1.000000")))
        (Components|StaticMesh|SetStaticMesh _returnvalue_2 (Variables|LaddetStepUp|GetLaddeSectionMesh))))
    (:then_2
      (Components|Box|SetBoxExtent (Variables|Default|GetPlayerClimbCheck) (Math|Vector|MakeVector _returnvalue _returnvalue (Math|Conversions|ToFloat(Integer) (/ (* (Variables|LaddetStepUp|GetNumberOfRungs) 56) 2))) true)
      (Transformation|SetRelativeLocation (Variables|Default|GetPlayerClimbCheck) (Math|Vector|MakeVector (Variables|LaddetStepUp|GetPlayerClimbCheckBoxOffSetX) 0.0 (+ (.z (.min (StaticMesh|GetBoundingBox (Variables|LaddetStepUp|GetLaddeSectionMesh)))) (/ (* (Variables|LaddetStepUp|GetNumberOfRungs) 56) 2))) false false))))