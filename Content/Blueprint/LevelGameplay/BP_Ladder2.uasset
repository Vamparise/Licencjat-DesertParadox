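; BP_Ladder2 is a modular ladder that lets the player climb while inside its trigger volume.
; The construction script stacks the selected mesh by segment count at a hardcoded spacing, then sizes and positions the PlayerClimbCheck box to match.
; The computed mesh height is not used for that spacing.
; Box begin and end overlaps call ToggleClimbing on BP_PlayerCharacter, passing the ladder as a reference.
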(event OnComponentBeginOverlap(PlayerClimbCheck)
  (params (OverlappedComponent :type Primitive%20Component%20Object%20Reference) (OtherActor :type Actor%20Object%20Reference) (OtherComp :type Primitive%20Component%20Object%20Reference) (OtherBodyIndex :type Integer) (bFromSweep :type Boolean) (SweepResult :type Hit%20Result%20Structure%20%28by%20ref%29))
  (bind _asbp_player_character (Utilities|Casting|CastToBP_PlayerCharacter OtherActor))
  (Default|ToggleClimbing _asbp_player_character true self))

(event OnComponentEndOverlap(PlayerClimbCheck)
  (params (OverlappedComponent :type Primitive%20Component%20Object%20Reference) (OtherActor :type Actor%20Object%20Reference) (OtherComp :type Primitive%20Component%20Object%20Reference) (OtherBodyIndex :type Integer))
  (bind _asbp_player_character (Utilities|Casting|CastToBP_PlayerCharacter OtherActor))
  (Default|ToggleClimbing _asbp_player_character false self))

(event EventBeginPlay)

(event Collision|EventActorBeginOverlap
  (params (OtherActor :type Actor%20Object%20Reference)))

(event EventTick
  (params (DeltaSeconds :type Float%20%28single-precision%29)))

(fn ConstructionScript
  (bind _playerclimbcheckboxsizexy (Variables|LaderStepUp|GetPlayerClimbCheckBoxSizeXY))
  (bind _returnvalue (/ _playerclimbcheckboxsizexy 2.0))
  (Utilities|FlowControl|Sequence
    (:then_0
      (Variables|LaderStepUp|SetLadder%20Selection%20Mesh%20Height (* (.z (.boxextent (StaticMesh|GetBounds (Variables|LaderStepUp|GetLadderSelectionMesh)))) 2.0)))
    (:then_1
      (for _index (range 0 (- (Variables|LaderStepUp|GetNumber%20of%20Runds) 1))
        (bind _returnvalue_2 (AddComponent|AddStaticMeshComponent false (Math|Transform|MakeTransform (Math|Vector|MakeVector 0.0 0.0 (Math|Conversions|ToFloat(Integer) (* _index 420))) "0, 0, 0" "1.000000,1.000000,1.000000")))
        (Components|StaticMesh|SetStaticMesh _returnvalue_2 (Variables|LaderStepUp|GetLadderSelectionMesh))))
    (:then_2
      (Components|Box|SetBoxExtent (Variables|LaderStepUp|GetPlayerClimbCheck) (Math|Vector|MakeVector _returnvalue _returnvalue (Math|Conversions|ToFloat(Integer) (/ (* (Variables|LaderStepUp|GetNumber%20of%20Runds) 420) 2))) true)
      (Transformation|SetRelativeLocation (Variables|LaderStepUp|GetPlayerClimbCheck) (Math|Vector|MakeVector (Variables|LaderStepUp|GetPlayer%20Climb%20Off%20Set%20X) 0.0 (+ (.z (.min (StaticMesh|GetBoundingBox (Variables|LaderStepUp|GetLadderSelectionMesh)))) (/ (* (Variables|LaderStepUp|GetNumber%20of%20Runds) 420) 2))) false false))))