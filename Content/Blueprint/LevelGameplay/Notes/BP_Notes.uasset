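; BP_Notes is a collectible note actor that highlights when approached and can be picked up.
; Its Sphere overlap applies an overlay material to the Cube, which is cleared on end overlap and at BeginPlay.
; PickUpItem prints a debug message, returns the item and note type, and triggers destruction after a short delay.
; Logic to show and remove a W_Notes widget is present but disconnected.
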(event OnComponentBeginOverlap(Sphere)
  (params (OverlappedComponent :type Primitive%20Component%20Object%20Reference) (OtherActor :type Actor%20Object%20Reference) (OtherComp :type Primitive%20Component%20Object%20Reference) (OtherBodyIndex :type Integer) (bFromSweep :type Boolean) (SweepResult :type Hit%20Result%20Structure%20%28by%20ref%29))
  (Rendering|Material|SetOverlayMaterial (Variables|Default|GetCube) (Variables|Default|GetOverlayMaterial) :!class /Script/Engine.MeshComponent))

(event OnComponentEndOverlap(Sphere)
  (params (OverlappedComponent :type Primitive%20Component%20Object%20Reference) (OtherActor :type Actor%20Object%20Reference) (OtherComp :type Primitive%20Component%20Object%20Reference) (OtherBodyIndex :type Integer))
  (Rendering|Material|SetOverlayMaterial (Variables|Default|GetCube) 0 :!class /Script/Engine.MeshComponent))

(event Custom|DestroyItem
  (Utilities|FlowControl|Delay 0.2)
  (Actor|DestroyActor))

(event EventBeginPlay
  (Rendering|Material|SetOverlayMaterial (Variables|Default|GetCube) 0 :!class /Script/Engine.MeshComponent))

(fn ConstructionScript)

(fn PickUpItem
  (Development|PrintString "Item Pick Up")
  (CallFunction|DestroyItem)
  (return (Variables|Default|GetItem) (Variables|Default|GetType%20Notes)))