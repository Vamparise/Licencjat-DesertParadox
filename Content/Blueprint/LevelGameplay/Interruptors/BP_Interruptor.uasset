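; BP_Interruptor is a pressure-plate switch for level gameplay that activates while something overlaps its Box.
; Begin overlap squashes and lowers the Button component and broadcasts OnInterruptorActivated.
; End overlap restores the raised button and broadcasts OnInterruptorDeactivated.
; Overlaps are neither filtered nor counted, as the player-character casts are disconnected, so any exit deactivates it.
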(event OnComponentBeginOverlap(Box)
  (params (OverlappedComponent :type Primitive%20Component%20Object%20Reference) (OtherActor :type Actor%20Object%20Reference) (OtherComp :type Primitive%20Component%20Object%20Reference) (OtherBodyIndex :type Integer) (bFromSweep :type Boolean) (SweepResult :type Hit%20Result%20Structure%20%28by%20ref%29))
  (CallFunction|ActiveButton))

(event OnComponentEndOverlap(Box)
  (params (OverlappedComponent :type Primitive%20Component%20Object%20Reference) (OtherActor :type Actor%20Object%20Reference) (OtherComp :type Primitive%20Component%20Object%20Reference) (OtherBodyIndex :type Integer))
  (CallFunction|DeactiveButton))

(event Custom|ActiveButton
  (Transformation|SetRelativeScale3D (Variables|Default|GetButton) "1.000000,1.000000,0.100000")
  (Transformation|SetRelativeLocation (Variables|Default|GetButton) "0.000000,0.000000,10.000000" false false)
  (Default|CallOnInterruptorActivated))

(event Custom|DeactiveButton
  (Transformation|SetRelativeScale3D (Variables|Default|GetButton) "1.000000,1.000000,0.500000")
  (Transformation|SetRelativeLocation (Variables|Default|GetButton) "0.000000,0.000000,30.000000" false false)
  (Default|CallOnInterruptorDeactivated))

(fn ConstructionScript)