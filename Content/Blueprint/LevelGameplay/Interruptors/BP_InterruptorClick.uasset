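; BP_InterruptorClick is a floor-button style switch for level gameplay that activates when something overlaps its Box trigger.
; Box overlap calls ActiveButtonClick, which squashes and lowers the ButtonClick component, then broadcasts OnClickActivated.
; End overlap calls DeactiveButtonClick, which is empty, so the button stays pressed.
; The logic that would raise it and broadcast OnClickDeactivated is disconnected and never runs.
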(event OnComponentBeginOverlap(Box)
  (params (OverlappedComponent :type Primitive%20Component%20Object%20Reference) (OtherActor :type Actor%20Object%20Reference) (OtherComp :type Primitive%20Component%20Object%20Reference) (OtherBodyIndex :type Integer) (bFromSweep :type Boolean) (SweepResult :type Hit%20Result%20Structure%20%28by%20ref%29))
  (CallFunction|ActiveButtonClick))

(event OnComponentEndOverlap(Box)
  (params (OverlappedComponent :type Primitive%20Component%20Object%20Reference) (OtherActor :type Actor%20Object%20Reference) (OtherComp :type Primitive%20Component%20Object%20Reference) (OtherBodyIndex :type Integer))
  (CallFunction|DeactiveButtonClick))

(event Custom|ActiveButtonClick
  (Transformation|SetRelativeScale3D (Variables|Default|GetButtonClick) "1.000000,1.000000,0.100000")
  (Transformation|SetRelativeLocation (Variables|Default|GetButtonClick) "0.000000,0.000000,10.000000" false false)
  (Default|CallOnClickActivated))

(event Custom|DeactiveButtonClick)

(fn ConstructionScript)