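; BP_GhostPlatform is a level platform that appears and disappears in response to an optional linked Sensor or Interuptor.
; A timeline scales the Cube's Y axis, playing forward to appear and reversing to disappear, which is also called on BeginPlay.
; Sensor pawn enter and leave events toggle it directly, while interruptor deactivation waits through a delay before hiding it.
; Item and interaction functions are stubs returning defaults.
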(event Custom|Appear
  (bind _scaletrack (Timeline|Timeline_AppearDissapear Play)
    (:Update
      (Transformation|SetWorldScale3D (Variables|Default|GetCube) (Math|Vector|MakeVector (Variables|Default|GetNew%20Scale%20X) (* _scaletrack 1e+01) (Variables|Default|GetNew%20Scale%20Z))))))

(event Custom|Dissappear
  (bind _scaletrack (Timeline|Timeline_AppearDissapear Reverse)
    (:Update
      (Transformation|SetWorldScale3D (Variables|Default|GetCube) (Math|Vector|MakeVector (Variables|Default|GetNew%20Scale%20X) (* _scaletrack 1e+01) (Variables|Default|GetNew%20Scale%20Z))))))

(event Custom|Pawn%20Enter
  ;[1 1 1] Sensor Activate
  (CallFunction|Appear))

(event Custom|Pawn%20Leave
  ;[1 1 1] Sensor Activate
  (CallFunction|Dissappear))

(event Custom|OnInterruptorActivated
  ;[1 1 1] Interruptor Activation
  (Utilities|FlowControl|Delay 0.0)
  (CallFunction|Appear))

(event Custom|OnInterruptorDeactivated
  ;[1 1 1] Interruptor Activation
  (Utilities|FlowControl|Delay 1e+01)
  (CallFunction|Dissappear))

(event EventBeginPlay
  (CallFunction|Dissappear)
  (Utilities|FlowControl|Sequence
    (:then_0
      ;[1 1 1] Sensor Activate
      (bind _sensor (Variables|Default|GetSensor)
        (:then
          (EventDispatchers|BindEventtoOnPawnEnter _sensor (delegate Custom|Pawn%20Enter))
          (EventDispatchers|BindEventtoOnPawnLeave _sensor (delegate Custom|Pawn%20Leave)))
        (:else)))
    (:then_1
      ;[1 1 1] Interruptor Activation
      (bind _interuptor (Variables|Activation|GetInteruptor)
        (:then
          (EventDispatchers|BindEventtoOnInterruptorActivated _interuptor (delegate Custom|OnInterruptorActivated))
          (EventDispatchers|BindEventtoOnInterruptorDeactivated _interuptor (delegate Custom|OnInterruptorDeactivated)))
        (:else)))))

(fn ConstructionScript)

(fn GetFractureBool
  (return false))

(fn GetItemType
  (return "NewEnumerator0"))

(fn GetMesh
  (return 0))

(fn Interactwith
  (params (CharacterINT :type BP%20Player%20Character%20Object%20Reference))
  (return false))