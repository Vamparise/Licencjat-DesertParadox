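; BP_BaseInterative is a base pickup that gives the player character a timed effect when they overlap its box.
; ApplyEffect and RemoveEffect are empty events, presumably for child Blueprints to override using the stored AffectedCharacter.
; On overlap it applies the effect, disables collision and hides the potion.
; After EffectDuration it removes the effect and restores both, so the pickup is reusable.
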(event OnComponentBeginOverlap(Box)
  (params (OverlappedComponent :type Primitive%20Component%20Object%20Reference) (OtherActor :type Actor%20Object%20Reference) (OtherComp :type Primitive%20Component%20Object%20Reference) (OtherBodyIndex :type Integer) (bFromSweep :type Boolean) (SweepResult :type Hit%20Result%20Structure%20%28by%20ref%29))
  ;[1 1 1] Overlap
  (bind _asbp_player_character (Utilities|Casting|CastToBP_PlayerCharacter OtherActor))
  (bind _output_get (Variables|Default|SetAffectedCharacter _asbp_player_character))
  (Utilities|IsValid _output_get
    (:Is%20Valid
      (CallFunction|ApplyEffect)
      (CallFunction|ConsumeInteractive)
      (Utilities|FlowControl|Delay (Variables|Default|GetEffect%20Duration))
      (CallFunction|RemoveEffect)
      (CallFunction|RestoreInteractive))))

(event Custom|ApplyEffect
  ;[1 1 1] Apply and Remove Effect
)

(event Custom|RemoveEffect
  ;[1 1 1] Apply and Remove Effect
)

(event Custom|ConsumeInteractive
  ;[1 1 1] Cosmetic Only
  (Collision|SetCollisionEnabled (Variables|Default|GetBox) "NoCollision")
  (Rendering|SetVisibility (Variables|Default|GetPotion) false false))

(event Custom|RestoreInteractive
  ;[1 1 1] Cosmetic Only
  (Collision|SetCollisionEnabled (Variables|Default|GetBox) "QueryOnly")
  (Rendering|SetVisibility (Variables|Default|GetPotion) true false))

(fn ConstructionScript)